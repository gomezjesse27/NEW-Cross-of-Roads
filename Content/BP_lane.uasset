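; Lane tile for a Crossy Road-style endless runner, configurable as grass, road, water or railroad.
; Setup functions set the mesh and either scatter trees and a coin or start looping timers spawning cars, logs, or trains with crossing lights.
; Player overlaps request new lanes from TunnelSpawner, count steps, or trigger drowning and game over on water.
; Edge triggers destroy passing traffic, and Tick removes the lane once the player is far past it.
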(event `self.StaticMeshComponent.OnComponentBeginOverlap`
  (params (OverlappedComponent :type "PrimitiveComponent Object Reference") (OtherActor :type "Actor Object Reference") (OtherComp :type "PrimitiveComponent Object Reference") (OtherBodyIndex :type Integer) (bFromSweep :type Boolean) (SweepResult :type "HitResult Structure (by ref)")))

(event `self.ReceiveBeginPlay`)

(event `self.ReceiveTick`
  (params (DeltaSeconds :type "Float (single-precision)"))
  (bind _returnvalue_x (`KismetMathLibrary.BreakVector` (`self.K2_GetActorLocation`)))
  (bind _returnvalue_x_2 (`KismetMathLibrary.BreakVector` (`self.K2_GetActorLocation` (`GameplayStatics.GetPlayerPawn` 0))))
  (if (< (- _returnvalue_x_2 _returnvalue_x) -50000.0)
    (`self.K2_DestroyActor`)))

(event `self.TrigggerZone.OnComponentBeginOverlap`
  (params (OverlappedComponent :type "PrimitiveComponent Object Reference") (OtherActor :type "Actor Object Reference") (OtherComp :type "PrimitiveComponent Object Reference") (OtherBodyIndex :type Integer) (bFromSweep :type Boolean) (SweepResult :type "HitResult Structure (by ref)"))
  (cast `/Game/ThirdPersonCharacter` OtherActor)
  (`/Game/BP_LaneSpawner.SpawnLaneAtSPawnPoint` (`self.Tunnel Spawner`))
  (`/Game/BP_LaneSpawner.Increment Shaped Collected` (`self.Tunnel Spawner`))
  (`ActorComponent.K2_DestroyComponent` (`self.TrigggerZone`)))

(event `self.TrigggerZonetodestroycaractor.OnComponentBeginOverlap`
  (params (OverlappedComponent :type "PrimitiveComponent Object Reference") (OtherActor :type "Actor Object Reference") (OtherComp :type "PrimitiveComponent Object Reference") (OtherBodyIndex :type Integer) (bFromSweep :type Boolean) (SweepResult :type "HitResult Structure (by ref)"))
  (bind _ascaractor (cast `/Game/caractor` OtherActor))
  (`self.K2_DestroyActor` _ascaractor))

(event `self.TrigggerZonecaractorfromleft.OnComponentBeginOverlap`
  (params (OverlappedComponent :type "PrimitiveComponent Object Reference") (OtherActor :type "Actor Object Reference") (OtherComp :type "PrimitiveComponent Object Reference") (OtherBodyIndex :type Integer) (bFromSweep :type Boolean) (SweepResult :type "HitResult Structure (by ref)"))
  (bind _ascaractorfromleft (cast `/Game/caractorfromleft` OtherActor))
  (`self.K2_DestroyActor` _ascaractorfromleft))

(event `self.TrigggerZonelogactorfromleft1.OnComponentBeginOverlap`
  (params (OverlappedComponent :type "PrimitiveComponent Object Reference") (OtherActor :type "Actor Object Reference") (OtherComp :type "PrimitiveComponent Object Reference") (OtherBodyIndex :type Integer) (bFromSweep :type Boolean) (SweepResult :type "HitResult Structure (by ref)"))
  (bind _aslogactorfromleft (cast `/Game/logactorfromleft` OtherActor))
  (`self.K2_DestroyActor` _aslogactorfromleft))

(event `self.TrigggerZonetodestroylogactor1.OnComponentBeginOverlap`
  (params (OverlappedComponent :type "PrimitiveComponent Object Reference") (OtherActor :type "Actor Object Reference") (OtherComp :type "PrimitiveComponent Object Reference") (OtherBodyIndex :type Integer) (bFromSweep :type Boolean) (SweepResult :type "HitResult Structure (by ref)"))
  (bind _aslogactor (cast `/Game/logactor` OtherActor))
  (`self.K2_DestroyActor` _aslogactor))

(event `self.waterdrown.OnComponentBeginOverlap`
  (params (OverlappedComponent :type "PrimitiveComponent Object Reference") (OtherActor :type "Actor Object Reference") (OtherComp :type "PrimitiveComponent Object Reference") (OtherBodyIndex :type Integer) (bFromSweep :type Boolean) (SweepResult :type "HitResult Structure (by ref)"))
  (if (`self.iswater`)
    (bind _asthird_person_character (cast `/Game/ThirdPersonCharacter` OtherActor))
    (`/Game/ThirdPersonCharacter.drown` _asthird_person_character)
    (bind _returnvalue (`|CreateWidget` "/Game/GameOver.GameOver_C"))
    (`UserWidget.AddToViewport` _returnvalue 0)
    (set `PlayerController.bShowMouseCursor` true (`GameplayStatics.GetPlayerController` 0))))

(event `self.STEPCOUNTER.OnComponentBeginOverlap`
  (params (OverlappedComponent :type "PrimitiveComponent Object Reference") (OtherActor :type "Actor Object Reference") (OtherComp :type "PrimitiveComponent Object Reference") (OtherBodyIndex :type Integer) (bFromSweep :type Boolean) (SweepResult :type "HitResult Structure (by ref)"))
  (bind _asthird_person_character (cast `/Game/ThirdPersonCharacter` OtherActor))
  (set `self.Chikref` _asthird_person_character)
  (`ActorComponent.K2_DestroyComponent` (`self.STEPCOUNTER`))
  (`/Game/ThirdPersonCharacter.increment steps` _asthird_person_character)
  (`KismetSystemLibrary.K2_SetTimer` null "checkindex" 3.0 true))

(event `self.czone.OnComponentBeginOverlap`
  (params (OverlappedComponent :type "PrimitiveComponent Object Reference") (OtherActor :type "Actor Object Reference") (OtherComp :type "PrimitiveComponent Object Reference") (OtherBodyIndex :type Integer) (bFromSweep :type Boolean) (SweepResult :type "HitResult Structure (by ref)"))
  (if (`self.can you destroycar`)
    (bind _ascaractor (cast `/Game/caractor` OtherActor))
    (`self.K2_DestroyActor` _ascaractor)
    (set `self.spawn?` false)
    (`KismetSystemLibrary.Delay` 2.0)))

(event `self.TrigggerZonetodestroyTRAINactor1.OnComponentBeginOverlap`
  (params (OverlappedComponent :type "PrimitiveComponent Object Reference") (OtherActor :type "Actor Object Reference") (OtherComp :type "PrimitiveComponent Object Reference") (OtherBodyIndex :type Integer) (bFromSweep :type Boolean) (SweepResult :type "HitResult Structure (by ref)"))
  (bind _astrainactor (cast `/Game/Trainactor` OtherActor))
  (`self.K2_DestroyActor` _astrainactor)
  (`/Game/traincross.TURNOFFIGHTS` (`self.TRAINCROSS1`))
  (`/Game/traincross.TURNOFFIGHTS` (`self.TRAINCROSS2`))
  (`/Game/traincross.TURNOFFIGHTS` (`self.TRAINCROSS3`))
  (set `self.ooping?` false))

(fn `checkindex`
  (if (> (- (`/Game/ThirdPersonCharacter.Steps collected` (`self.Chikref`)) (`self.laneindexbplane`)) 2)
    (set `self.can you destroycar` true)))

(fn `RANDOM`
  (`StaticMeshComponent.SetStaticMesh` (`self.StaticMesh`) (select `int` (`KismetMathLibrary.RandomIntegerInRange` 0 10) :`0` "/Game/railroad_vox.railroad_vox" :`1` "/Game/1lane_grass_dark_vox.1lane_grass_dark_vox" :`2` "/Game/1lane_grass_dark_vox.1lane_grass_dark_vox" :`3` "/Game/1lane_grass_dark_vox.1lane_grass_dark_vox" :`4` "/Game/1lane_grass_dark_vox.1lane_grass_dark_vox" :`5` "/Game/1lane_water_vox.1lane_water_vox" :`6` "/Game/1lane_water_vox.1lane_water_vox" :`7` "/Game/1lane_grass_vox.1lane_grass_vox" :`8` "/Game/1lane_grass_vox.1lane_grass_vox" :`9` "/Game/1lane_grass_vox.1lane_grass_vox" :`10` "/Game/1lane_grass_vox.1lane_grass_vox" :!type "StaticMesh Object Reference")))

(fn `Setgrass`
  (bind _staticmesh (`self.StaticMesh`))
  (bind _returnvalue (`SceneComponent.K2_GetComponentLocation` (`self.start`)))
  (bind _returnvalue_2 (`SceneComponent.K2_GetComponentLocation` (`self.end`)))
  (bind (_returnvalue_x _returnvalue_y) (`KismetMathLibrary.BreakVector` (`SceneComponent.K2_GetComponentLocation` (`self.coinstart`))))
  (bind (_returnvalue_x_2 _returnvalue_y_2 _returnvalue_z) (`KismetMathLibrary.BreakVector` (`SceneComponent.K2_GetComponentLocation` (`self.coinend`))))
  (bind _returnvalue_3 (`SceneComponent.K2_GetComponentLocation` (`self.start`)))
  (bind _returnvalue_4 (`SceneComponent.K2_GetComponentLocation` (`self.end`)))
  (bind (_returnvalue_x_3 _returnvalue_y_3) (`KismetMathLibrary.BreakVector` (`SceneComponent.K2_GetComponentLocation` (`self.coinstart`))))
  (bind (_returnvalue_x_4 _returnvalue_y_4 _returnvalue_z_2) (`KismetMathLibrary.BreakVector` (`SceneComponent.K2_GetComponentLocation` (`self.coinend`))))
  ;[1 1 1] I basically placed a spawn point at the edge of the map and got a random float between those 2 locations to randomly place 20 trees down. Their is code in the tree actors that doesnt let them overlap, basically just if they overlap one gets destroyed. I laso placed big trees on the grass strips where the chicken cannot go passed.
  (if (`/Game/BP_LaneSpawner.alternating grass` (`self.Tunnel Spawner`))
    (set `/Game/BP_LaneSpawner.alternating grass` false (`self.Tunnel Spawner`))
    (`StaticMeshComponent.SetStaticMesh` _staticmesh "/Game/1lane_grass_dark_vox.1lane_grass_dark_vox")
    (bind _returnvalue_5 (`|SpawnActorFromClass` "/Game/Coin.Coin_C" (`KismetMathLibrary.MakeTransform` (`KismetMathLibrary.MakeVector` _returnvalue_x (`KismetMathLibrary.RandomFloatInRange` _returnvalue_y _returnvalue_y_2) _returnvalue_z)) "Undefined" "OverrideRootScale" null null))
    ;;[1 1 1] random y in between x and z
    (set `self.mycoin` _returnvalue_5)
    (`|SpawnActorFromClass` "/Game/tree.tree_C" (`KismetMathLibrary.MakeTransform` _returnvalue) "Undefined" "OverrideRootScale" null null)
    (`|SpawnActorFromClass` "/Game/tree.tree_C" (`KismetMathLibrary.MakeTransform` _returnvalue_2) "Undefined" "OverrideRootScale" null null)
    (bind _output_get (set `self.startlocation` _returnvalue))
    (bind _output_get_2 (set `self.endlocation` _returnvalue_2))
    (for _ (range 21)
      (bind _returnvalue_6 (`|SpawnActorFromClass` "/Game/tree.tree_C" (`KismetMathLibrary.MakeTransform` (`KismetMathLibrary.MakeVector` (.x _output_get) (`KismetMathLibrary.RandomFloatInRange` (.y _output_get) (.y _output_get_2)) (.z _output_get))) "Undefined" "OverrideRootScale" null null))
      (bind _output_get_3 (set `self.treenew` _returnvalue_6))
      (`/Game/tree.random` _output_get_3))
    (else
      (`StaticMeshComponent.SetStaticMesh` _staticmesh "/Game/1lane_grass_vox.1lane_grass_vox")
      (set `/Game/BP_LaneSpawner.alternating grass` true (`self.Tunnel Spawner`))
      (bind _returnvalue_7 (`|SpawnActorFromClass` "/Game/Coin.Coin_C" (`KismetMathLibrary.MakeTransform` (`KismetMathLibrary.MakeVector` _returnvalue_x_3 (`KismetMathLibrary.RandomFloatInRange` _returnvalue_y_3 _returnvalue_y_4) _returnvalue_z_2)) "Undefined" "OverrideRootScale" null null))
      (set `self.mycoin` _returnvalue_7)
      (`|SpawnActorFromClass` "/Game/tree.tree_C" (`KismetMathLibrary.MakeTransform` _returnvalue_3) "Undefined" "OverrideRootScale" null null)
      (`|SpawnActorFromClass` "/Game/tree.tree_C" (`KismetMathLibrary.MakeTransform` _returnvalue_4) "Undefined" "OverrideRootScale" null null)
      (bind _output_get_4 (set `self.startlocation` _returnvalue_3))
      (bind _output_get_5 (set `self.endlocation` _returnvalue_4))
      (for _ (range 6)
        (bind _returnvalue_8 (`|SpawnActorFromClass` "/Game/tree.tree_C" (`KismetMathLibrary.MakeTransform` (`KismetMathLibrary.MakeVector` (.x _output_get_4) (`KismetMathLibrary.RandomFloatInRange` (.y _output_get_4) (.y _output_get_5)) (.z _output_get_4))) "Undefined" "OverrideRootScale" null null))
        (bind _output_get_6 (set `self.treenew` _returnvalue_8))
        (`/Game/tree.random` _output_get_6)))))

(fn `SetRailroad`
  (`StaticMeshComponent.SetStaticMesh` (`self.StaticMesh`) "/Game/railroad_vox.railroad_vox")
  (bind _returnvalue (`|SpawnActorFromClass` "/Game/traincross.traincross_C" (`KismetMathLibrary.Conv_VectorToTransform` (`SceneComponent.K2_GetComponentLocation` (`self.rrcrossingspawn`))) "Undefined" "OverrideRootScale" null null))
  (set `self.TRAINCROSS1` _returnvalue)
  (bind _returnvalue_2 (`|SpawnActorFromClass` "/Game/traincross.traincross_C" (`KismetMathLibrary.Conv_VectorToTransform` (`SceneComponent.K2_GetComponentLocation` (`self.rrcrossingspawn1`))) "Undefined" "OverrideRootScale" null null))
  (set `self.TRAINCROSS2` _returnvalue_2)
  (bind _returnvalue_3 (`|SpawnActorFromClass` "/Game/traincross.traincross_C" (`KismetMathLibrary.Conv_VectorToTransform` (`SceneComponent.K2_GetComponentLocation` (`self.rrcrossingspawn2`))) "Undefined" "OverrideRootScale" null null))
  (set `self.TRAINCROSS3` _returnvalue_3)
  (`KismetSystemLibrary.K2_SetTimer` null "spawntrain" (`KismetMathLibrary.RandomFloatInRange` 8.0 30.0) true))

(fn `Setroad`
  (`StaticMeshComponent.SetStaticMesh` (`self.StaticMesh`) "/Game/roadmemake.roadmemake")
  (set `self.istrue` (`KismetMathLibrary.RandomBool`))
  (if (`self.istrue`)
    (`KismetSystemLibrary.K2_SetTimer` null "spawnactor" 3.0 true)
    (else
      (`KismetSystemLibrary.K2_SetTimer` null "spawnactorleft" 3.0 true))))

(fn `SetWater`
  (set `self.iswater` true)
  (`StaticMeshComponent.SetStaticMesh` (`self.StaticMesh1`) "/Game/1lane_water_vox.1lane_water_vox")
  (set `self.istrue2` (`KismetMathLibrary.RandomBool`))
  (if (`self.istrue2`)
    (`KismetSystemLibrary.K2_SetTimer` null "spawnlog" 7.0 true)
    (else
      (`KismetSystemLibrary.K2_SetTimer` null "spawnlogfromleft" 7.0 true))))

(fn `spawnactor`
  ;[1 1 1] Working
  (if (`self.spawn?`)
    (bind _returnvalue (`|SpawnActorFromClass` "/Game/caractor.caractor_C" (`KismetMathLibrary.MakeTransform` (`SceneComponent.K2_GetComponentLocation` (`self.end`))) "Undefined" "OverrideRootScale" null null))
    (`/Game/caractor.randomcar` _returnvalue)
    (`/Game/caractor.changespeedfunction` _returnvalue (`KismetMathLibrary.RandomFloatInRange` -10000.0 -30000.0))))

(fn `spawnactorleft`
  (if (`self.spawn?`)
    (bind _returnvalue (`|SpawnActorFromClass` "/Game/caractorfromleft.caractorfromleft_C" (`KismetMathLibrary.MakeTransform` (`SceneComponent.K2_GetComponentLocation` (`self.start`))) "Undefined" "OverrideRootScale" null null))
    (`/Game/caractorfromleft.randomcar2` _returnvalue)
    (`/Game/caractorfromleft.changespeedfunction2` _returnvalue (`KismetMathLibrary.RandomFloatInRange` 10000.0 30000.0))))

(fn `spawnlog`
  (`|SpawnActorFromClass` "/Game/logactor.logactor_C" (`KismetMathLibrary.MakeTransform` (`SceneComponent.K2_GetComponentLocation` (`self.end`))) "Undefined" "OverrideRootScale" null null))

(fn `spawnlogfromleft`
  (`|SpawnActorFromClass` "/Game/logactorfromleft.logactorfromleft_C" (`KismetMathLibrary.MakeTransform` (`SceneComponent.K2_GetComponentLocation` (`self.start`))) "Undefined" "OverrideRootScale" null null))

(fn `Spawntrain`
  (bind _traincross3 (`self.TRAINCROSS3`))
  (for _ (range 6)
    (`KismetSystemLibrary.K2_SetTimer` (`self.TRAINCROSS1`) "Alternatelights" 1.0)
    (`KismetSystemLibrary.K2_SetTimer` (`self.TRAINCROSS2`) "Alternatelights" 1.0)
    (`KismetSystemLibrary.K2_SetTimer` _traincross3 "Alternatelights" 1.0))
  ;[1 1 1] Working
  (`/Game/traincross.TURNONLIGHTS` _traincross3)
  (`/Game/traincross.TURNONLIGHTS` (`self.TRAINCROSS2`))
  (`/Game/traincross.TURNONLIGHTS` (`self.TRAINCROSS1`))
  (bind _returnvalue (`|SpawnActorFromClass` "/Game/Trainactor.Trainactor_C" (`KismetMathLibrary.MakeTransform` (`SceneComponent.K2_GetComponentLocation` (`self.end`))) "Undefined" "OverrideRootScale" null null))
  (`/Game/Trainactor.changespeedfunction` _returnvalue (`KismetMathLibrary.RandomFloatInRange` -50000.0 -100000.0)))

(fn `spawntrees`
  (`|SpawnActorFromClass` "/Game/oaktreeee.oaktreeee_C" (`KismetMathLibrary.MakeTransform` (`SceneComponent.K2_GetComponentLocation` (`self.Scene`))) "Undefined" "OverrideRootScale" null null)
  (`|SpawnActorFromClass` "/Game/oaktreeee.oaktreeee_C" (`KismetMathLibrary.MakeTransform` (`SceneComponent.K2_GetComponentLocation` (`self.Scene1`))) "Undefined" "OverrideRootScale" null null))

(fn `UserConstructionScript`)