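; Player pawn Blueprint (bp_chicky) with mouse look and axis-driven movement, set up to collect coins.
; Movement input scaled by MaxSpeed is consumed each Tick and applied as a local offset, without delta time or sweep.
; Coin overlaps call IncrementCoinsCollected, which is empty, and the mesh hit event only casts to caractor.
; The CoinScore widget creation and counter update nodes are disconnected and never run.
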(event `self.ReceiveActorBeginOverlap`
  (params (OtherActor :type "Actor Object Reference"))
  (cast `/Game/Coin` OtherActor)
  (`self.IncrementCoinsCollected`))

(event `self.ReceiveBeginPlay`)

(event `InputAxis|Turn Right / Left Mouse`
  (params (AxisValue :type "Float (single-precision)"))
  (`self.AddControllerYawInput` AxisValue))

(event `InputAxis|Look Up / Down Mouse`
  (params (AxisValue :type "Float (single-precision)"))
  (`self.AddControllerPitchInput` AxisValue))

(event `InputAxis|Move Forward / Backward`
  (params (AxisValue :type "Float (single-precision)"))
  (`self.AddMovementInput` (`self.GetActorForwardVector`) (* AxisValue (`self.maxSpeed`))))

(event `InputAxis|Move Right / Left`
  (params (AxisValue :type "Float (single-precision)"))
  (`self.AddMovementInput` (`self.GetActorRightVector`) (* AxisValue (`self.maxSpeed`))))

(event `self.ReceiveTick`
  (params (DeltaSeconds :type "Float (single-precision)"))
  (bind _returnvalue (`self.ConsumeMovementInputVector`))
  (`self.K2_AddActorLocalOffset` _returnvalue))

(event `self.StaticMesh.OnComponentHit`
  (params (HitComponent :type "PrimitiveComponent Object Reference") (OtherActor :type "Actor Object Reference") (OtherComp :type "PrimitiveComponent Object Reference") (NormalImpulse :type "Vector Structure") (Hit :type "HitResult Structure (by ref)"))
  (cast `/Game/caractor` OtherActor))

(fn `IncrementCoinsCollected`)

(fn `UserConstructionScript`)