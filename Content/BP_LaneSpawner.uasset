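; Lane spawner actor that builds a chain of BP_lane actors, with water, railroad, grass-with-trees and road types.
; On BeginPlay it places a first lane at a fixed location, then chains untyped lanes from each newest lane's SpawnPoint.
; SpawnLaneAtSPawnPoint makes a weighted random type pick for the newest lane before spawning the next.
; Each spawned lane receives an incrementing index and a reference back to the spawner.
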(event `self.ReceiveBeginPlay`
  (`self.Spawn Initial Lanes`))

(fn `Increment Shaped Collected`)

(fn `Spawn Initial Lanes`
  (for _ (range 11)
    (`/Engine/EditorBlueprintResources/StandardMacros.IsValid` (`self.Newest Lane`)
      (:`Is Valid`
        (`self.SpawnLaneAtSPawnPoint_0`))
      (:`Is Not Valid`
        (`self.SpawnLane` (-8590.0 150.0 35520.0))))))

(fn `SpawnLane`
  (params (SpawnLocation :type "Vector Structure"))
  (locals (NewLocalVar_0 :type "/Game/BP_lane Object Reference"))
  (bind _result (`/Engine/EditorBlueprintResources/StandardMacros.IncrementInt` (`self.laneIndex`))
    (:`  `
      (bind _output_get (set `self.laneIndex` _result))
      (bind _returnvalue (`|SpawnActorFromClass` "/Game/BP_lane.BP_lane_C" (`KismetMathLibrary.MakeTransform` SpawnLocation) "Undefined" "OverrideRootScale" null null))
      (set `/Game/BP_lane.laneindexbplane` _output_get _returnvalue)
      (bind _output_get_2 (set `self.Newest Lane` _returnvalue))
      (set `/Game/BP_lane.Tunnel Spawner` self _output_get_2))))

(fn `SpawnLaneAtSPawnPoint`
  (bind _newest_lane (`self.Newest Lane`))
  (switch `int` (`KismetMathLibrary.RandomInteger` 16)
    (:`0`
      (`/Game/BP_lane.SetWater` _newest_lane :!label _label))
    (:`1`
      (`/Game/BP_lane.SetRailroad` _newest_lane))
    (:`2`
      (`/Game/BP_lane.Setgrass` _newest_lane :!label _label_2)
      (`/Game/BP_lane.spawntrees` _newest_lane))
    (:`3`
      (goto _label_2))
    (:`4`
      (goto _label_2))
    (:`5`
      (goto _label))
    (:`6`
      (goto _label))
    (:`7`
      (`/Game/BP_lane.Setroad` _newest_lane :!label _label_3))
    (:`8`
      (goto _label_3))
    (:`9`
      (goto _label))
    (:`10`
      (goto _label))
    (:`11`
      (goto _label_3))
    (:`12`
      (goto _label_3))
    (:`13`
      (goto _label_3))
    (:`14`
      (goto _label_3))
    (:`15`
      (goto _label_3))
    (:`16`
      (goto _label_3)))
  (`self.SpawnLane` (`SceneComponent.K2_GetComponentLocation` (`/Game/BP_lane.Spawn Point` _newest_lane))))

(fn `SpawnLaneAtSPawnPoint_0`
  (`self.SpawnLane` (`SceneComponent.K2_GetComponentLocation` (`/Game/BP_lane.Spawn Point` (`self.Newest Lane`)))))

(fn `SpawnRandomLane_0`
  (params (SpawnLocation :type "Vector Structure"))
  (locals (NewLocalVar_0 :type "/Game/BP_lane Object Reference"))
  (switch `int` (`KismetMathLibrary.RandomIntegerInRange` 0 3)))

(fn `UserConstructionScript`)