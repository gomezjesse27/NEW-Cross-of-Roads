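; BP_river is a river segment actor that extends the level by spawning copies of itself as the chicky advances.
; When a bp_chicky overlaps TriggerZone, it spawns another BP_river at the SpawnPoint component's world location, so segments chain together.
; The trigger has no once-only guard and nothing here destroys old segments.
; An unconnected leftover chain spawns at the player pawn's location using a Lane1 reference and never runs.
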(event `self.ReceiveBeginPlay`)

(event `self.TrigggerZone.OnComponentBeginOverlap`
  (params (OverlappedComponent :type "PrimitiveComponent Object Reference") (OtherActor :type "Actor Object Reference") (OtherComp :type "PrimitiveComponent Object Reference") (OtherBodyIndex :type Integer) (bFromSweep :type Boolean) (SweepResult :type "HitResult Structure (by ref)"))
  (cast `/Game/bp_chicky` OtherActor)
  (`|SpawnActorFromClass` "BP_river_C" (`KismetMathLibrary.MakeTransform` (`SceneComponent.K2_GetComponentLocation` (`self.Spawn Point`))) "Undefined" "OverrideRootScale" null null))

(fn `UserConstructionScript`
  (`parent.UserConstructionScript`))